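; Main menu character for a local player slot that joins on any key press while MenuGameMode is waiting.
; Joining registers the controller with the game mode and spawns a parameter widget offset by controller ID, removed on return to mode selection.
; Team and nickname cycle with wraparound, recursively skipping unavailable nicknames and freeing the previous one.
; The first key pressed flags keyboard or gamepad use; only non-keyboard players cycle choices through gameplay input actions.
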(event `Key|AnyKey` :consume false
  (params (Key :type "Key Structure"))
  ;[0.9277 0.6737 1] Listen for connection
  (:`Pressed`
    (if (not (`self.connected`))
      (set `self.useKeyboard` (or (`KismetInputLibrary.Key_IsKeyboardKey` Key) (`KismetInputLibrary.Key_IsMouseButton` Key)))
      (bind _asmenu_game_mode (cast `MenuGameMode` (`GameplayStatics.GetGameMode`)))
      (if (`MenuGameMode.waiting` _asmenu_game_mode)
        (bind _asplayer_controller (cast `PlayerController` (`self.GetController`)))
        (`MenuGameMode.SetPlayer` _asmenu_game_mode _asplayer_controller)
        (`self.Connect`)))))

(event `self.ReceiveBeginPlay`
  ;[1 0.9124 0.7625] BeginPlay
  (bind _asmenu_game_mode (cast `MenuGameMode` (`GameplayStatics.GetGameMode`)))
  (add `MenuGameMode.OnGoToModeSelection` _asmenu_game_mode (delegate `BackToMenu`)))

(event `BackToMenu`
  ;[1 0.9124 0.7625] BeginPlay
  (if (`self.connected`)
    (`Widget.RemoveFromParent` (`self.widgetRef`))
    (set `self.connected` false)
    (bind _asplayer_controller (cast `PlayerController` (`self.GetController`)))
    (`self.K2_SetActorLocation` (`KismetMathLibrary.MakeVector` -300.0 (* (`GameplayStatics.GetPlayerControllerID` _asplayer_controller) -100.0) 200.0))))

(event `Connect`
  ;[0.6508 1 0.899] Connect (Appear on screen)
  (`|ExecutionSequence`
    (:`then_0`
      (set `self.connected` true)
      (bind _asmenu_game_mode (cast `MenuGameMode` (`GameplayStatics.GetGameMode`)))
      (`self.ChangeNickname` 1)
      (set `self.team` (`|GetArrayItem` (`MenuGameMode.teamList` _asmenu_game_mode) (`self.teamID`))))
    (:`then_1`
      (bind _asplayer_controller (cast `PlayerController` (`self.GetController`)))
      (bind _returnvalue (`|CreateWidget` "/Game/Widgets/MainMenu/WidgetPlayerParameters.WidgetPlayerParameters_C"))
      (bind _output_get (set `self.widgetRef` _returnvalue))
      (`/Game/Widgets/MainMenu/WidgetPlayerParameters.GoToSelf` _output_get self)
      (`Widget.SetRenderTranslation` (`/Game/Widgets/MainMenu/WidgetPlayerParameters.ButtonCanvas` _output_get) (`KismetMathLibrary.MakeVector2D` (* (`GameplayStatics.GetPlayerControllerID` _asplayer_controller) 450.0))))))

(event `FocusOnWidget`
  ;[0.6508 1 0.899] Connect (Appear on screen)
)

(event `ChangeTeam`
  (params (step :type Integer :default 1))
  ;[1 0.6685 0.9101] Setup parameters
  (bind _asmenu_game_mode (cast `MenuGameMode` (`GameplayStatics.GetGameMode`)))
  (bind _teamlist (`MenuGameMode.teamList` _asmenu_game_mode))
  (bind _id (`self.GetNextID` (`self.teamID`) (`KismetArrayLibrary.Array_Length` _teamlist) step))
  (bind _output_get (set `self.teamID` _id))
  (set `self.team` (`|GetArrayItem` _teamlist _output_get)))

(event `ChangeNickname`
  (params (step :type Integer :default 1))
  ;[1 0.6685 0.9101] Setup parameters
  (bind _asmenu_game_mode (cast `MenuGameMode` (`GameplayStatics.GetGameMode`)))
  (bind _id (`self.GetNextID` (`self.nicknameID`) (`KismetArrayLibrary.Array_Length` (`MenuGameMode.nicknameList` _asmenu_game_mode)) step))
  (bind _output_get (set `self.nicknameID` _id))
  (bind (_nickname _returnvalue) (`MenuGameMode.TryGetNickname` _asmenu_game_mode _output_get))
  (if _returnvalue
    (`MenuGameMode.FreeNickname` _asmenu_game_mode (`self.lastNicknameID`))
    (set `self.lastNicknameID` _output_get)
    (set `self.nickName` _nickname)
    (else
      (`self.ChangeNickname` step))))

(event `InputAction|Aim`
  (params (Key :type "Key Structure"))
  (:`Pressed`
    (if (and (not (`self.useKeyboard`)) (`self.connected`))
      (`self.ChangeNickname` -1))))

(event `InputAction|Fire`
  (params (Key :type "Key Structure"))
  (:`Pressed`
    (if (and (not (`self.useKeyboard`)) (`self.connected`))
      (`self.ChangeNickname` 1))))

(event `InputAction|Sprint`
  (params (Key :type "Key Structure"))
  (:`Pressed`
    (if (and (not (`self.useKeyboard`)) (`self.connected`))
      (`self.ChangeTeam` -1))))

(event `InputAction|Ultime`
  (params (Key :type "Key Structure"))
  (:`Pressed`
    (if (and (not (`self.useKeyboard`)) (`self.connected`))
      (`self.ChangeTeam` 1))))

(fn `GetNextID`
  (params (curID :type Integer) (lenght :type Integer) (step :type Integer :default 1))
  (returns (ID :type Integer))
  (bind _returnvalue (+ curID step))
  (if (>= _returnvalue lenght)
    (return 0)
    (elif (< _returnvalue 0)
      (return (- lenght 1))
      (else
        (return _returnvalue)))))

(fn `UserConstructionScript`)