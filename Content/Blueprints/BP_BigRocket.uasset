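; BP_BigRocket is a large rocket projectile that trails smoke and sets off a big explosion.
; A looping timer from BeginPlay rapidly spawns BP_SmokeRocket at the particle spawn point, while the parent BeginPlay call is left unconnected.
; The OnExplosion binding spawns BP_BigExplosion there with a wide camera shake and a randomly low-pitched sound.
; Hits attach a temporary impact decal to the struck component, aligned to the surface normal.
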(event `CustomEvent_1`
  (`|SpawnActorFromClass` "/Game/Blueprints/BP_SmokeRocket.BP_SmokeRocket_C" (`KismetMathLibrary.MakeTransform` (`SceneComponent.K2_GetComponentLocation` (`self.ParticlSpawnPoint`))) "Undefined" "OverrideRootScale" null null))

(event `self.ReceiveBeginPlay`
  (add `Rocket.OnExplosion` (delegate `CustomEvent`))
  (`KismetSystemLibrary.K2_SetTimerDelegate` (delegate `CustomEvent_1`) 0.02 true))

(event `CustomEvent`
  (bind _returnvalue (`SceneComponent.K2_GetComponentLocation` (`self.ParticlSpawnPoint`)))
  (`|SpawnActorFromClass` "/Game/Blueprints/BP_BigExplosion.BP_BigExplosion_C" (`KismetMathLibrary.MakeTransform` _returnvalue) "Undefined" "OverrideRootScale" null null)
  (`GameplayStatics.PlayWorldCameraShake` "/Game/Blueprints/Shake/BigShake.BigShake_C" _returnvalue 0.0 5000.0)
  (`GameplayStatics.PlaySoundAtLocation` "/Game/Sounds/explosion.explosion" (0.0 0.0 0.0) (struct) 1.5 (`KismetMathLibrary.RandomFloatInRange` 0.6 0.8) 0.0 null null null))

(event `self.ReceiveHit`
  (params (MyComp :type "PrimitiveComponent Object Reference") (Other :type "Actor Object Reference") (OtherComp :type "PrimitiveComponent Object Reference") (bSelfMoved :type Boolean) (HitLocation :type "Vector Structure") (HitNormal :type "Vector Structure") (NormalImpulse :type "Vector Structure") (Hit :type "HitResult Structure (by ref)"))
  (`GameplayStatics.SpawnDecalAttached` "/Game/Materials/M_Impact.M_Impact" (300.0 300.0 300.0) OtherComp "None" HitLocation (`KismetMathLibrary.MakeRotFromX` HitNormal) "KeepWorldPosition" 60.0))

(fn `UserConstructionScript`
  (`parent.UserConstructionScript`))