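; BP_NickNameManager sets up overhead nickname labels for every pair of players on BeginPlay.
; Each viewing character gets a NickNameUpdater, and every other character gets a screen-space WidgetComponent owned by that viewer's local player, allowing separate labels per viewer.
; Labels show the nickname in team color, start hidden, and are registered with the viewer's updater.
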(event `self.ReceiveBeginPlay`
  ;[1 1 1] The player that should see the nicknames
  (for _array_element (`self.GetEveryPlayers`)
    (bind _asthird_person_character (cast `/Game/Blueprints/ThirdPersonCharacter` _array_element))
    (bind _returnvalue (`AddComponent|NODE_AddNickNameUpdater-0` :`self` _asthird_person_character))
    (bind _asplayer_controller (cast `PlayerController` (`Pawn.GetController` _asthird_person_character)))
    ;[1 1 1] The showed player
    (for _array_element_2 (`self.GetEveryPlayers`)
      (bind _asthird_person_character_2 (cast `/Game/Blueprints/ThirdPersonCharacter` _array_element_2))
      (if (not (== _asthird_person_character_2 _asthird_person_character))
        (bind _returnvalue_2 (`|CreateWidget` "/Game/Widgets/WidgetNickName.WidgetNickName_C" _asplayer_controller))
        (bind _returnvalue_3 (`AddComponent|NODE_AddWidgetComponent-2` :`self` _asthird_person_character_2 :`RelativeTransform` (`KismetMathLibrary.MakeTransform` (0.0 0.0 110.0))))
        ;;[1 1 1] Setting the widget component
        (`WidgetComponent.SetWidget` _returnvalue_3 _returnvalue_2)
        (`WidgetComponent.SetWidgetSpace` _returnvalue_3 "Screen")
        (`WidgetComponent.SetDrawAtDesiredSize` _returnvalue_3 true)
        (`PrimitiveComponent.SetCollisionEnabled` _returnvalue_3 "NoCollision")
        (`WidgetComponent.SetOwnerPlayer` _returnvalue_3 (`Widget.GetOwningLocalPlayer` _returnvalue_2))
        (`SceneComponent.SetVisibility` _returnvalue_3 false false)
        (`NickNameUpdater.AddWidgetForPlayer` _returnvalue _returnvalue_3 _asthird_person_character_2)
        (bind _nickname (`/Game/Widgets/WidgetNickName.Nickname` _returnvalue_2))
        ;;[1 1 1] Setting the text (nickname)
        (`TextBlock.SetText` _nickname (`KismetTextLibrary.Conv_StringToText` (`DeathRocket_ProtoCharacter.GetNickName` _asthird_person_character_2)))
        (`TextBlock.SetColorAndOpacity` _nickname (make `SlateColor` (`KismetMathLibrary.Conv_ColorToLinearColor` (`DeathRocket_ProtoCharacter.GetTeam` _asthird_person_character_2))))))))

(fn `UserConstructionScript`)