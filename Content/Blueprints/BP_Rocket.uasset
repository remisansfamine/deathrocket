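; BP_Rocket is a rocket projectile that leaves a smoke trail and explodes in its shooter's team color.
; A fast looping timer spawns BP_SmokeRocket actors at the particle spawn point.
; The OnExplosion callback plays a world camera shake and spawns BP_PoofExplosion, tinting its Niagara effect with the team color and a slightly brighter variant.
; The Hit event is empty, and its impact decal logic is disconnected.
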(event `self.ReceiveBeginPlay`
  (add `self.OnExplosion` (delegate `ExplosionCallback`))
  (`KismetSystemLibrary.K2_SetTimerDelegate` (delegate `Spawn particle`) 0.02 true))

(event `Spawn particle`
  (`|SpawnActorFromClass` "/Game/Blueprints/BP_SmokeRocket.BP_SmokeRocket_C" (`KismetMathLibrary.MakeTransform` (`SceneComponent.K2_GetComponentLocation` (`self.ParticlSpawnPoint`))) "Undefined" "OverrideRootScale" null null))

(event `ExplosionCallback`
  (bind _returnvalue (`self.K2_GetActorLocation`))
  (bind _returnvalue_2 (`KismetMathLibrary.Conv_ColorToLinearColor` (`DeathRocket_ProtoCharacter.team` (`self.shooter`))))
  (`GameplayStatics.PlayWorldCameraShake` "/Game/Blueprints/Shake/Shake.Shake_C" _returnvalue 0.0 2500.0)
  (bind _returnvalue_3 (`|SpawnActorFromClass` "/Game/Blueprints/BP_PoofExplosion.BP_PoofExplosion_C" (`KismetMathLibrary.MakeTransform` _returnvalue) "Undefined" "OverrideRootScale" null null))
  (bind _niagara (`/Game/Blueprints/BP_PoofExplosion.Niagara` _returnvalue_3))
  (`FXSystemComponent.SetColorParameter` _niagara "Color_01" _returnvalue_2)
  (`FXSystemComponent.SetColorParameter` _niagara "Color_02" (+ _returnvalue_2 (* (`KismetMathLibrary.LinearColor_White`) 0.1))))

(event `self.ReceiveHit`
  (params (MyComp :type "PrimitiveComponent Object Reference") (Other :type "Actor Object Reference") (OtherComp :type "PrimitiveComponent Object Reference") (bSelfMoved :type Boolean) (HitLocation :type "Vector Structure") (HitNormal :type "Vector Structure") (NormalImpulse :type "Vector Structure") (Hit :type "HitResult Structure (by ref)")))

(fn `UserConstructionScript`)