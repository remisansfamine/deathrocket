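; Game instance for DeathRocket that stores per-player parameters taken from the menu characters.
; Init pre-fills the PlayerParams array with one entry per player slot.
; SetPlayerParameters walks that array, casts each indexed player pawn to MenuCharacter and writes its connection state, team and nickname into the matching entry.
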(event `self.ReceiveInit`
  ;[1 0.5322 0.6223] Init
  (for _ (range 5)
    (`KismetArrayLibrary.Array_Add` (`self.playerParams`))))

(event `SetPlayerParameters`
  ;[1 0.9473 0.5916] Player Parameters
  (for _index (range (+ (`KismetArrayLibrary.Array_Length` (`self.playerParams`)) 1))
    (bind _asmenu_character (cast `/Game/Blueprints/MainMenu/MenuCharacter` (`GameplayStatics.GetPlayerPawn` _index)))
    (`KismetArrayLibrary.Array_Set` (`self.playerParams`) _index (make `/Game/Structures/PlayerParams` (`/Game/Blueprints/MainMenu/MenuCharacter.connected` _asmenu_character) (`/Game/Blueprints/MainMenu/MenuCharacter.team` _asmenu_character) (`/Game/Blueprints/MainMenu/MenuCharacter.nickName` _asmenu_character)))))