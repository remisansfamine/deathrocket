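; Score manager that shows and hides a scoreboard widget on a player's screen.
; On BeginPlay it binds handlers to OnDisplay and OnHide events, each requiring the query to be a PlayerController.
; Display creates a new score widget for that controller, stores it on Scoreboard and adds it to the player's screen.
; Hide removes whichever widget Scoreboard currently holds, regardless of which controller asked.
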(event `DisplayScoreboard` :!signature `self.OnDisplay`
  (params (query :type "Controller Object Reference"))
  ;[1 1 1] Display
  (bind _asplayer_controller (cast `PlayerController` query))
  (bind _returnvalue (`|CreateWidget` "/Game/Widgets/WidgetScore.WidgetScore_C" _asplayer_controller))
  (`WidgetComponent.SetWidget` (`self.Scoreboard`) _returnvalue)
  (`UserWidget.AddToPlayerScreen` _returnvalue 0))

(event `self.ReceiveBeginPlay`
  (`|ExecutionSequence`
    (:`then_0`
      ;[1 1 1] Display
      (add `self.OnDisplay` (delegate `DisplayScoreboard`)))
    (:`then_1`
      ;[1 1 1] Hide
      (add `self.OnHide` (delegate `HideScoreboard`)))))

(event `HideScoreboard` :!signature `self.OnHide`
  (params (query :type "Controller Object Reference"))
  ;[1 1 1] Hide
  (cast `PlayerController` query)
  (`Widget.RemoveFromParent` (`WidgetComponent.GetWidget` (`self.Scoreboard`))))

(fn `UserConstructionScript`)