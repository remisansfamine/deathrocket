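; BP_LittleRocket is a small rocket with a smoke trail, an explosion effect and impact marks.
; On BeginPlay it starts a fast looping timer that spawns BP_SmokeRocket actors at its particle spawn point, and binds to OnExplosion.
; The explosion callback spawns a poof explosion and plays a world camera shake at the mesh location.
; Hits attach a temporary impact decal to the struck component, oriented by the hit normal.
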(event `self.ReceiveBeginPlay`
  (add `self.OnExplosion` (delegate `ExplosionCallback`))
  (`KismetSystemLibrary.K2_SetTimerDelegate` (delegate `Spawn particle`) 0.02 true))

(event `Spawn particle`
  (`|SpawnActorFromClass` "/Game/Blueprints/BP_SmokeRocket.BP_SmokeRocket_C" (`KismetMathLibrary.MakeTransform` (`SceneComponent.K2_GetComponentLocation` (`self.ParticlSpawnPoint`))) "Undefined" "OverrideRootScale" null null))

(event `ExplosionCallback`
  (bind _returnvalue (`SceneComponent.K2_GetComponentLocation` (`self.RocketMesh`)))
  (`|SpawnActorFromClass` "/Game/Blueprints/BP_LittlePoofExplosion.BP_LittlePoofExplosion_C" (`KismetMathLibrary.MakeTransform` _returnvalue) "Undefined" "OverrideRootScale" null null)
  (`GameplayStatics.PlayWorldCameraShake` "/Game/Blueprints/Shake/LittleShake.LittleShake_C" _returnvalue 0.0 2500.0))

(event `self.ReceiveHit`
  (params (MyComp :type "PrimitiveComponent Object Reference") (Other :type "Actor Object Reference") (OtherComp :type "PrimitiveComponent Object Reference") (bSelfMoved :type Boolean) (HitLocation :type "Vector Structure") (HitNormal :type "Vector Structure") (NormalImpulse :type "Vector Structure") (Hit :type "HitResult Structure (by ref)"))
  (`GameplayStatics.SpawnDecalAttached` "/Game/Materials/M_Impact.M_Impact" (30.0 30.0 30.0) OtherComp "None" HitLocation (`KismetMathLibrary.MakeRotFromX` HitNormal) "KeepWorldPosition" 60.0))

(fn `UserConstructionScript`)