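; BP_RocketMenu is a rocket actor, apparently for the menu, that flies forward and leaves a smoke trail.
; On BeginPlay it applies a one-time impulse to its GFX component along the actor's forward vector.
; A looping timer rapidly spawns BP_SmokeRocket actors at the ParticlSpawnPoint component's location.
; The rocket destroys itself after a short delay.
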(event `self.ReceiveBeginPlay`
  (`PrimitiveComponent.AddImpulse` (`self.GFX`) (* (`self.GetActorForwardVector`) 50000.0) "None" false)
  (`KismetSystemLibrary.K2_SetTimerDelegate` (delegate `Spawn particle`) 0.02 true)
  (`KismetSystemLibrary.Delay` 3.0)
  (`self.K2_DestroyActor`))

(event `Spawn particle`
  (`|SpawnActorFromClass` "/Game/Blueprints/BP_SmokeRocket.BP_SmokeRocket_C" (`KismetMathLibrary.MakeTransform` (`SceneComponent.K2_GetComponentLocation` (`self.ParticlSpawnPoint`))) "Undefined" "OverrideRootScale" null null))

(fn `UserConstructionScript`)