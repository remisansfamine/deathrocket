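; Rocket actor that leaves a smoke trail and produces a visual blast when it explodes.
; A fast looping timer started on BeginPlay spawns smoke actors at the particle spawn point.
; A callback bound to the OnExplosion event spawns a poof explosion at the rocket's location and plays a radial world camera shake.
; The Hit event only prints a debug string.
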(event `self.ReceiveBeginPlay`
  (add `self.OnExplosion` (delegate `ExplosionCallback`))
  (`KismetSystemLibrary.K2_SetTimerDelegate` (delegate `Spawn particle`) 0.02 true))

(event `Spawn particle`
  (`|SpawnActorFromClass` "/Game/Blueprints/BP_SmokeRocket.BP_SmokeRocket_C" (`KismetMathLibrary.MakeTransform` (`SceneComponent.K2_GetComponentLocation` (`self.ParticlSpawnPoint`))) "Undefined" "OverrideRootScale" null null))

(event `ExplosionCallback`
  (bind _returnvalue (`self.K2_GetActorLocation`))
  (`|SpawnActorFromClass` "/Game/Blueprints/BP_PoofExplosion.BP_PoofExplosion_C" (`KismetMathLibrary.MakeTransform` _returnvalue) "Undefined" "OverrideRootScale" null null)
  (`GameplayStatics.PlayWorldCameraShake` "/Game/Blueprints/Shake/Shake.Shake_C" _returnvalue 0.0 2500.0))

(event `self.ReceiveHit`
  (params (MyComp :type "PrimitiveComponent Object Reference") (Other :type "Actor Object Reference") (OtherComp :type "PrimitiveComponent Object Reference") (bSelfMoved :type Boolean) (HitLocation :type "Vector Structure") (HitNormal :type "Vector Structure") (NormalImpulse :type "Vector Structure") (Hit :type "HitResult Structure (by ref)"))
  (`KismetSystemLibrary.PrintString` "Hello"))

(fn `UserConstructionScript`)